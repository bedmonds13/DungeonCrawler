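; Play-mode game mode that spawns the saved player character and manages troll spawning for a dungeon level.
; BeginPlay loads BP_DungeonSaveGame, spawns the selected character at the first PlayerStart found, possesses it and restores saved health.
; Each SpawnEnemyWave call spawns one troll at a random BP_SpawnManager point while counts are below the cap.
; Otherwise, when no current enemies remain, it unlocks every BP_Door.
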(event EventBeginPlay
  (bind _outactors (Actor|GetAllActorsOfClass "/Script/Engine.PlayerStart"))
  (bind _returnvalue (SaveGame|LoadGamefromSlot "SaveSlot"))
  (bind _asbp_dungeon_save_game (Utilities|Casting|CastToBP_DungeonSaveGame _returnvalue))
  (bind _returnvalue_2 (Game|SpawnActorfromClass (.playerselectedcharacter (Variables|/Game/Blueprints/BP_DungeonSaveGame.BP_DungeonSaveGame_C|GetCurrentCharacterStats _asbp_dungeon_save_game)) (Math|Transform|MakeTransform (Transformation|GetActorLocation (Utilities|Array|Get(acopy) _outactors)) "0, 0, 0" "1,1,1") "Undefined" 0 0))
  (Pawn|Possess (Game|GetPlayerController 0) _returnvalue_2)
  (Class|DungeonCharacter|SetCharacterHealth _returnvalue_2 (.health (Variables|/Game/Blueprints/BP_DungeonSaveGame.BP_DungeonSaveGame_C|GetCurrentCharacterStats _asbp_dungeon_save_game))))

(event EventTick
  (params (DeltaSeconds :type Float%20%28single-precision%29)))

(fn ConstructionScript)

(fn SpawnEnemyWave
  (if (and (> (Variables|Default|GetMaxEnemyCount) (Variables|Default|GetCurrentEnemyCount)) (< (Variables|Default|GetTotalEnemyCount) (Variables|Default|GetMaxEnemyCount)))
    (bind _outactors (Actor|GetAllActorsOfClass "/Game/Blueprints/BP_SpawnManager.BP_SpawnManager_C"))
    (bind _spawnpoint (Default|GetRandomSpawnPoint (Utilities|Array|Get(acopy) _outactors)))
    (Game|SpawnActorfromClass "/Game/Blueprints/Characters/BP_AI_Troll.BP_AI_Troll_C" (Math|Transform|MakeTransform _spawnpoint "0, 0, 0" "1,1,1") "AdjustIfPossibleButDontSpawnIfColliding" 0 0)
    (Math|Integer|IncrementInt (Variables|Default|GetTotalEnemyCount))
    (elif (< (Variables|Default|GetCurrentEnemyCount) 1)
      (Development|PrintString "Defeated all enemies")
      (CallFunction|UnlockNext:evels))))

(fn UnlockNext:evels
  (bind _outactors (Actor|GetAllActorsOfClass "/Game/Blueprints/BP_Door.BP_Door_C"))
  (for _array_element _outactors
    (Variables|/Game/Blueprints/BP_Door.BP_Door_C|SetDoorLocked _array_element false)))