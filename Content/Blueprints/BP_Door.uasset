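; Dungeon door that saves the player's character state and loads the level named by LevelName when walked into.
; Actor overlap prints a message if DoorLocked is set; otherwise OpenDoor proceeds only for a DungeonCharacter owned by a DungeonPlayerController.
; OpenDoor writes Health and character class into a newly created BP_DungeonSaveGame in "SaveSlot", then opens the level.
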(event Collision|EventActorBeginOverlap
  (params (OtherActor :type Actor%20Object%20Reference))
  (if (Variables|Default|GetDoorLocked)
    (Development|PrintString "Door locked")
    (else
      (CallFunction|OpenDoor OtherActor))))

(event EventTick
  (params (DeltaSeconds :type Float%20%28single-precision%29)))

(fn ConstructionScript)

(fn OpenDoor
  (params (Character :type Actor%20Object%20Reference))
  (bind _asdungeon_character (Utilities|Casting|CastToDungeonCharacter Character))
  (Utilities|Casting|CastToDungeonPlayerController (Components|GetOwner _asdungeon_character))
  (bind _returnvalue (SaveGame|CreateSaveGameObject "/Game/Blueprints/BP_DungeonSaveGame.BP_DungeonSaveGame_C"))
  (Variables|/Game/Blueprints/BP_DungeonSaveGame.BP_DungeonSaveGame_C|SetCurrentCharacterStats _returnvalue (Utilities|Struct|MakeCharacterStats (Variables|/Script/DungeonCrawler.DungeonCharacter|Gethealth _asdungeon_character) (Utilities|GetClass _asdungeon_character)))
  (SaveGame|SaveGametoSlot _returnvalue "SaveSlot")
  (Development|PrintString "Game state saved")
  (Game|OpenLevel(byName) (Variables|Default|GetLevelName)))