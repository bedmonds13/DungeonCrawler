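; Anim notify state that runs the dragon's flame attack for the span it covers in an animation.
; On begin it casts the mesh owner to BP_Dragon, sets IsAttacking, and starts the flame Niagara effect and sound.
; On end it clears IsAttacking, deactivates the effect and stops the sound.
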(fn ReceivedNotifyBegin
  (params (MeshComp :type Skeletal%20Mesh%20Component%20Object%20Reference) (Animation :type Anim%20Sequence%20Base%20Object%20Reference) (TotalDuration :type Float%20%28single-precision%29))
  (bind _asbp_dragon (Utilities|Casting|CastToBP_Dragon (Components|GetOwner MeshComp)))
  (Variables|/Game/Blueprints/Characters/BP_Dragon.BP_Dragon_C|SetIsAttacking _asbp_dragon true)
  (Components|Activation|Activate (Variables|/Game/Blueprints/Characters/BP_Dragon.BP_Dragon_C|GetFlameNiagraActor _asbp_dragon) false)
  (Audio|Components|Audio|Play (Variables|/Game/Blueprints/Characters/BP_Dragon.BP_Dragon_C|GetFlameSound _asbp_dragon) 0.0))

(fn ReceivedNotifyEnd
  (params (MeshComp :type Skeletal%20Mesh%20Component%20Object%20Reference) (Animation :type Anim%20Sequence%20Base%20Object%20Reference))
  (bind _asbp_dragon (Utilities|Casting|CastToBP_Dragon (Components|GetOwner MeshComp)))
  (Variables|/Game/Blueprints/Characters/BP_Dragon.BP_Dragon_C|SetIsAttacking _asbp_dragon false)
  (Components|Activation|Deactivate (Variables|/Game/Blueprints/Characters/BP_Dragon.BP_Dragon_C|GetFlameNiagraActor _asbp_dragon))
  (Audio|Components|Audio|Stop (Variables|/Game/Blueprints/Characters/BP_Dragon.BP_Dragon_C|GetFlameSound _asbp_dragon))
  (return true))