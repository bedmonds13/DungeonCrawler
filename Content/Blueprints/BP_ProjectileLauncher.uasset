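; BP_ProjectileLauncher is a launcher actor that fires BP_FireRock projectiles at random intervals.
; Tick runs into a randomized Delay, which paces the repeated launches without a timer.
; Each shot picks a force between MinLaunchForce and MaxLaunchForce and sets the LaunchPoint pitch to Angle, keeping roll and yaw.
; It then spawns the rock at LaunchPoint, passing forward vector times force as StartVelocity.
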(event EventBeginPlay)

(event EventTick
  (params (DeltaSeconds :type Float%20%28single-precision%29))
  (bind _angle (Variables|Default|GetAngle))
  (bind _launchpoint (Variables|Default|GetLaunchPoint))
  (bind _returnvalue (Transformation|GetWorldRotation _launchpoint))
  (bind _returnvalue_2 (Math|Rotator|MakeRotator (.roll _returnvalue) _angle (.yaw _returnvalue)))
  (Utilities|FlowControl|Delay (Math|Random|RandomFloatinRange 1.0 1e+01))
  (Variables|Default|SetLaunch%20Force (Math|Random|RandomFloatinRange (Variables|Default|GetMinLaunchForce) (Variables|Default|GetMaxLaunchForce)))
  (Transformation|SetWorldRotation _launchpoint _returnvalue_2 false false)
  (Variables|Default|SetStart%20Velocity (* (Math|Vector|GetForwardVector _launchpoint) (Variables|Default|GetLaunch%20Force)))
  (Game|SpawnActorfromClass "/Game/Blueprints/BP_FireRock.BP_FireRock_C" (Math|Transform|MakeTransform (Transformation|GetWorldLocation _launchpoint) _returnvalue_2) "Undefined" 0 (Variables|Default|GetStart%20Velocity) 0))

(fn ConstructionScript)