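; BP_FireRock is a physics-driven lava ball projectile that damages the player or spawns a BP_Floor where it meets the floor.
; On BeginPlay it launches the Lavaball component at StartVelocity.
; An actor overlap with the player's pawn sends a Light TakeHitMessage with Damage, then destroys the rock.
; A Lavaball overlap with a component tagged Floor spawns BP_Floor at the ball's location, then destroys the rock.
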(event OnComponentBeginOverlap(Lavaball)
  (params (OverlappedComponent :type Primitive%20Component%20Object%20Reference) (OtherActor :type Actor%20Object%20Reference) (OtherComp :type Primitive%20Component%20Object%20Reference) (OtherBodyIndex :type Integer) (bFromSweep :type Boolean) (SweepResult :type Hit%20Result%20Structure%20%28by%20ref%29))
  (if (Components|ComponentHasTag OtherComp (Utilities|Name|MakeLiteralName "Floor"))
    (Game|SpawnActorfromClass "/Game/Blueprints/BP_Floor.BP_Floor_C" (Math|Transform|MakeTransform (Transformation|GetWorldLocation (Variables|Default|GetLavaball))) "AdjustIfPossibleButAlwaysSpawn" 0 0)
    (Actor|DestroyActor)))

(event EventBeginPlay
  (Physics|SetPhysicsLinearVelocity (Variables|Default|GetLavaball) (Variables|Default|GetStart%20Velocity) false "None"))

(event EventTick
  (params (DeltaSeconds :type Float%20%28single-precision%29)))

(event Collision|EventActorBeginOverlap
  (params (OtherActor :type Actor%20Object%20Reference))
  (bind _returnvalue (Game|GetPlayerController 0))
  (bind _returnvalue_2 (Pawn|GetControlledPawn _returnvalue))
  (if (== _returnvalue_2 OtherActor)
    (Class|ITakeHit|TakeHit(Message) _returnvalue_2 (Variables|Default|GetDamage) 0 "Light")
    (Actor|DestroyActor)))

(fn ConstructionScript)