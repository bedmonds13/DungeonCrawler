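; Warrior is a melee player character with a dual-blade axe, overriding parent attack, special move, dodge and hit handling.
; Attacks play montages gated by CanAttack, and separate impact events run debug-drawn sphere overlaps at the axe to deal light or heavy hits.
; The special move also launches struck DungeonCharacters.
; Dodge becomes a cursor-facing block that, against frontal hits, knocks the Warrior back and returns damage to the attacker after parent hit handling.
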(event EventBeginPlay)

(event Collision|EventActorBeginOverlap
  (params (OtherActor :type Actor%20Object%20Reference)))

(event EventTick
  (params (DeltaSeconds :type Float%20%28single-precision%29)))

(event EventAttack
  (params (newRotation :type Rotator :default "0, 0, 0"))
  (bind _attackmontages (Variables|Default|GetattackMontages))
  (bind _returnvalue (Utilities|Array|Length _attackmontages))
  (bind _returnvalue_2 (- _returnvalue 1))
  (bind _returnvalue_3 (Math|Random|RandomIntegerinRange 0 _returnvalue_2))
  (bind _output (Utilities|Array|Get(acopy) _attackmontages _returnvalue_3))
  ;[1 1 1] Attack and Impact Event
  (|CallParentFunction newRotation)
  (if (Variables|Default|GetCanAttack)
    (Variables|Default|SetCanAttack false)
    (Variables|Default|SetmaxInputDelayCount (Variables|/Script/Engine.AnimSequenceBase|GetSequenceLength _output))
    (Animation|Montage|PlayMontage (Variables|Character|GetMesh) _output 1.5
      (:OnBlendOut
        (Variables|Default|SetCanAttack true)))))

(event EventTakeHit
  (params (damage :type Float%20%28single-precision%29) (attackingCharacter :type Dungeon%20Character%20Object%20Reference) (type :type AttackType%20Enum :default "Light"))
  (bind _returnvalue (Transformation|GetActorLocation attackingCharacter))
  (bind _returnvalue_2 (Transformation|GetActorRotation))
  (bind _returnvalue_3 (Transformation|GetActorLocation))
  (bind _isblocking (Variables|Default|GetIsBlocking))
  (bind _returnvalue_4 (- _returnvalue _returnvalue_3))
  (bind _returnvalue_5 (Math|Vector|GetForwardVector _returnvalue_2))
  (bind _returnvalue_6 (Math|Vector|DotProduct _returnvalue_4 _returnvalue_5))
  (bind _returnvalue_7 (> _returnvalue_6 0.0))
  (bind _returnvalue_8 (and _isblocking _returnvalue_7))
  ;[1 1 1] Take Hit Interface override
  (|CallParentFunction damage attackingCharacter type)
  (switch Utilities|FlowControl|Switch|SwitchonAttackType type
    (:Light
      (if _returnvalue_8
        (Character|LaunchCharacter (* _returnvalue_4 -10) false false :!label _label)
        (Class|ITakeHit|TakeHit attackingCharacter damage self type)
        (Animation|PlayAnimMontage "/Game/Animations/Warrior/Standing_Block_react_Montage.Standing_Block_react_Montage" 1.0 "None")))
    (:Heavy
      (if _returnvalue_8
        (goto _label)))))

(event EventAttackImpactEvent
  (bind _dual_blade_axe16 (Variables|Default|GetDual_Blade_Axe16))
  (bind _returnvalue (Transformation|GetWorldLocation _dual_blade_axe16))
  ;[1 1 1] Attack and Impact Event
  (bind _outactors (Collision|SphereOverlapActors _returnvalue 5e+01 (Utilities|Array|MakeArray "ObjectTypeQuery3") 0 (Utilities|Array|MakeArray self)))
  (Rendering|Debug|DrawDebugSphere _returnvalue 5e+01 12 "(R=0.000000,G=0.061501,B=1.000000,A=1.000000)" 1.0 1e+01)
  (for _array_element _outactors
    (Class|AISenseDamage|ReportDamageEvent _array_element self 0.0 _returnvalue)
    (Class|ITakeHit|TakeHit(Message) _array_element 1.0 self "Light")))

(event EventSpecialMove
  (params (newRotation :type Rotator :default "0, 0, 0"))
  (bind _specialattackmontage (Variables|Default|GetSpecialAttackMontage))
  ;[1 1 1] Special Move and Impact
  (|CallParentFunction (Math|Rotator|MakeRotator (.roll newRotation) (.pitch newRotation) (.yaw newRotation)))
  (if (Variables|Default|GetCanAttack)
    (Variables|Default|SetCanAttack false)
    (Transformation|SetActorRotation (Math|Rotator|MakeRotator 0.0 0.0 (.yaw newRotation)))
    (Variables|Default|SetmaxInputDelayCount (Variables|/Script/Engine.AnimSequenceBase|GetSequenceLength _specialattackmontage))
    (Animation|Montage|PlayMontage (Variables|Character|GetMesh) _specialattackmontage 1.5
      (:OnBlendOut
        (Variables|Default|SetCanAttack true)))))

(event EventSpecialImpactEvent
  (bind _dual_blade_axe16 (Variables|Default|GetDual_Blade_Axe16))
  (bind _specialmoveforce (Variables|Default|GetSpecialMoveForce))
  (bind _returnvalue (Transformation|GetSocketLocation _dual_blade_axe16 "Top"))
  ;[1 1 1] Special Move and Impact
  (bind _outactors (Collision|SphereOverlapActors _returnvalue (Variables|Default|GetSpecialMoveRadius) (Utilities|Array|MakeArray "ObjectTypeQuery3") 0 (Utilities|Array|MakeArray self)))
  (Rendering|Debug|DrawDebugSphere _returnvalue (Variables|Default|GetSpecialMoveRadius) 12 "(R=0.000000,G=0.004274,B=1.000000,A=1.000000)" 1.0 2e+01)
  (for _array_element _outactors
    (Development|PrintString (Utilities|GetDisplayName _array_element))
    (Class|ITakeHit|TakeHit(Message) _array_element 3.0 self "Heavy")
    (bind _asdungeon_character (Utilities|Casting|CastToDungeonCharacter _array_element))
    (Character|LaunchCharacter _asdungeon_character (Math|Vector|MakeVector (* (.x (* (Math|Vector|Normalize (Math|Vector|GetForwardVector (Variables|/Script/Engine.Character|GetCapsuleComponent _asdungeon_character))) (Math|Vector|Normalize (- (Transformation|GetActorLocation _array_element) (Transformation|GetActorLocation))))) _specialmoveforce) (* (.y (* (Math|Vector|Normalize (Math|Vector|GetForwardVector (Variables|/Script/Engine.Character|GetCapsuleComponent _asdungeon_character))) (Math|Vector|Normalize (- (Transformation|GetActorLocation _array_element) (Transformation|GetActorLocation))))) _specialmoveforce) 1e+02) false false)))

(event Input|ActionEvents|InputActionDodge
  (params (Key :type Key%20Structure :default "None"))
  (bind _returnvalue (Transformation|GetActorRotation))
  ;[1 1 1] Dodge/Block override
  (:Pressed
    (Variables|Default|SetIsBlocking true)
    (Variables|Default|SetCanAttack false)
    (bind _asdungeon_player_controller (Utilities|Casting|CastToDungeonPlayerController (Pawn|GetController)))
    (Transformation|SetActorRotation (Math|Rotator|MakeRotator (.roll _returnvalue) (.pitch _returnvalue) (.yaw (Math|Rotator|FindLookatRotation (Transformation|GetActorLocation) (.location (.HitResult (Game|Player|GetHitResultUnderCursorbyChannel _asdungeon_player_controller "TraceTypeQuery1" true)))))))
    (Class|DungeonCharacter|ResetInputTimer)
    (Default|CallBlockingEventDispatcher (Variables|Default|GetIsBlocking) :!label _label))
  (:Released
    (Variables|Default|SetIsBlocking false)
    (Variables|Default|SetCanAttack true)
    (Utilities|Casting|CastToDungeonPlayerController (Pawn|GetController))
    (goto _label)))

(fn ConstructionScript)