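; Dragon combat character that plays random hit-reaction and attack montages, with melee impacts damaging a player-controlled DungeonCharacter via sphere overlap.
; Its fire-breath special repeats forward sphere traces while attacking, damaging DungeonCharacters from a head-attached flamethrower effect, which spawns inactive with stopped audio at BeginPlay.
; CustomMoveTo stores a synchronous nav path that GetDesiredMovement follows point by point as a direction vector.
; Debug spheres, traces and prints remain throughout.
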(event Custom|CustomMoveTo
  (params (MoveToLocation :type Vector))
  (bind _returnvalue (Class|NavigationSystemV1|FindPathtoLocationSynchronously (Transformation|GetActorLocation) MoveToLocation 0 0))
  (bind _output_get (Variables|Default|SetNav%20Path%20Points (Variables|/Script/NavigationSystem.NavigationPath|GetPathPoints _returnvalue)))
  (for _array_element _output_get
    (Rendering|Debug|DrawDebugSphere (Math|Vector|MakeVector (.x _array_element) (.y _array_element) 4e+02) 1e+02 12 "(R=0.053875,G=0.000000,B=1.000000,A=1.000000)" 1.0 1.0)
    (Variables|Default|SetAIMoving true)))

(event Collision|EventActorBeginOverlap
  (params (OtherActor :type Actor%20Object%20Reference)))

(event EventTick
  (params (DeltaSeconds :type Float%20%28single-precision%29)))

(event EventTakeHit
  (params (damage :type Float%20%28single-precision%29) (attackingCharacter :type Dungeon%20Character%20Object%20Reference) (type :type AttackType%20Enum :default "Light"))
  (bind _mesh (Variables|Character|GetMesh))
  (|CallParentFunction damage attackingCharacter type)
  (switch int (Math|Random|RandomIntegerinRange 0 2)
    (:Default
      (Animation|Montage|PlayMontage _mesh "/Game/Animations/Dragon/Dragon_HitRight.Dragon_HitRight" :!label _label
        (:then
          _)))
    (:0
      (Animation|Montage|PlayMontage _mesh "/Game/Animations/Dragon/Dragon_HitFront.Dragon_HitFront"
        (:then
          _)))
    (:1
      (Animation|Montage|PlayMontage _mesh "/Game/Animations/Dragon/Dragon_HitLeft.Dragon_HitLeft"
        (:then
          _)))
    (:2
      (goto _label)))
  (Development|PrintString "Dragon hit"))

(event EventAttack
  (params (newRotation :type Rotator :default "0, 0, 0"))
  (bind _attackmontages (Variables|Default|GetattackMontages))
  (Animation|Montage|PlayMontage (Variables|Character|GetMesh) (Utilities|Array|Get(acopy) _attackmontages (Math|Random|RandomIntegerinRange 0 (- (Utilities|Array|Length _attackmontages) 1)))))

(event EventAttackImpactEvent
  (bind _attackpoint (Variables|Components|GetAttackPoint))
  (bind _returnvalue (Transformation|GetWorldLocation _attackpoint))
  (bind _outactors (Collision|SphereOverlapActors _returnvalue 1e+02 (Utilities|Array|MakeArray "ObjectTypeQuery3") 0))
  (bind _array_element (Utilities|Array|ForEachLoopwithBreak _outactors :!label _label)
    (:LoopBody
      (Rendering|Debug|DrawDebugSphere _returnvalue 1e+02 12 "(R=1.000000,G=1.000000,B=1.000000,A=1.000000)" 1.0 5.0)
      (bind _asdungeon_character (Utilities|Casting|CastToDungeonCharacter _array_element))
      (Utilities|Casting|CastToDungeonPlayerController (Pawn|GetController _asdungeon_character))
      (Class|ITakeHit|TakeHit(Message) _asdungeon_character (Variables|Default|GetDamage) self "Light")
      (Development|PrintString (Utilities|GetDisplayName _asdungeon_character))
      (goto _label Break))))

(event EventSpecialMove
  (params (newRotation :type Rotator :default "0, 0, 0"))
  (bind _flameniagraactor (Variables|Components|GetFlameNiagraActor))
  (bind _returnvalue (Transformation|GetWorldLocation _flameniagraactor))
  (Animation|Montage|PlayMontage (Variables|Character|GetMesh) "/Game/QuadrapedCreatures/MountainDragon/Animations/DRAGON_spreadFire_AnimMon.DRAGON_spreadFire_AnimMon"
    (:then
      (Utilities|FlowControl|Delay 0.44 :!label _label)
      (Utilities|FlowControl|Sequence
        (:then_0
          (if (Variables|Default|GetIsAttacking)
            (goto _label)))
        (:then_1
          (bind _outhits (Collision|MultiSphereTraceForObjects _returnvalue (+ _returnvalue (* (Math|Vector|GetForwardVector (Transformation|GetWorldRotation _flameniagraactor)) 5e+02)) 0.0 (Utilities|Array|MakeArray "ObjectTypeQuery3") false 0 "Persistent"))
          (for _array_element _outhits
            (bind _asdungeon_character (Utilities|Casting|CastToDungeonCharacter (.HitActor (Collision|BreakHitResult _array_element))))
            (Class|ITakeHit|TakeHit _asdungeon_character (Variables|Default|GetDamage) self "Light")))))))

(event EventBeginPlay
  (bind _returnvalue (Niagara|SpawnSystemAttached "/Game/Niagara/NS_Flamethrower.NS_Flamethrower" (Variables|Character|GetMesh) "MOUNTAIN_DRAGON_-Head" "0, 0, 0" "0,-75.000000,0.000000" "KeepRelativeOffset" false false "ManualRelease"))
  (bind _output_get (Variables|Components|SetFlameNiagraActor _returnvalue))
  (bind _returnvalue_2 (Audio|SpawnSoundAttached "/Game/Sounds/Dragon_with_Fire_1_-_QuickSounds_com.Dragon_with_Fire_1_-_QuickSounds_com" _output_get "None" "0, 0, 0" "0, 0, 0" "KeepRelativeOffset" true 1.0 1.0 0.0 0 0 false))
  (bind _output_get_2 (Variables|Default|SetFlameSound _returnvalue_2))
  (Audio|Components|Audio|Stop _output_get_2))

(fn ConstructionScript)

(fn GetDesiredMovement
  (bind _returnvalue (Transformation|GetActorLocation))
  (bind _nav_path_points (Variables|Default|GetNav%20Path%20Points))
  (if (Variables|Default|GetAIMoving)
    (if (<= (Variables|Default|GetNav%20Path%20Index) (Utilities|Array|LastIndex _nav_path_points))
      (if (< (Math|Vector|Distance(Vector) (Utilities|Array|Get(acopy) _nav_path_points (Variables|Default|GetNav%20Path%20Index)) _returnvalue) (Variables|Default|GetAcceptance%20Radius))
        (Math|Integer|IncrementInt (Variables|Default|GetNav%20Path%20Index))
        (else
          (return (Math|Vector|GetUnitDirection(Vector) _returnvalue (Utilities|Array|Get(acopy) _nav_path_points (Variables|Default|GetNav%20Path%20Index))))))
      (else
        (Variables|Default|SetAIMoving false)
        (Variables|Default|SetNav%20Path%20Index 0)
        (return "0, 0, 0")))))

(fn GetDesiredRotation
  (params (NewParam :type Rotator)))